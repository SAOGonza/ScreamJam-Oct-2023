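; Interactable button actor that opens every Door4_BP whose Door4Value matches its Button4Value.
; A Box overlap with BP_ThirdPersonCharacter opens a gate for the Interact input, enabled at BeginPlay.
; Pressing plays a click and lerps the button inward via the ButtonIn timeline, then back out via ButtonOut played in reverse.
; The door search and OpenDoor4 call run on every ButtonOut update, not once on completion.
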(event OnComponentBeginOverlap(Box)
  (params (OverlappedComponent :type Primitive%20Component%20Object%20Reference) (OtherActor :type Actor%20Object%20Reference) (OtherComp :type Primitive%20Component%20Object%20Reference) (OtherBodyIndex :type Integer) (bFromSweep :type Boolean) (SweepResult :type Hit%20Result%20Structure%20%28by%20ref%29))
  ;[1 1 1] Button Interaction
  (Utilities|Casting|CastToBP_ThirdPersonCharacter OtherActor)
  (Utilities|FlowControl|Gate true) ; enters at Open
)

(event OnComponentEndOverlap(Box)
  (params (OverlappedComponent :type Primitive%20Component%20Object%20Reference) (OtherActor :type Actor%20Object%20Reference) (OtherComp :type Primitive%20Component%20Object%20Reference) (OtherBodyIndex :type Integer))
  ;[1 1 1] Button Interaction
  (Utilities|Casting|CastToBP_ThirdPersonCharacter OtherActor)
  (Utilities|FlowControl|Gate true) ; enters at Close
)

(event EventBeginPlay
  (bind _button4 (Variables|Default|GetButton4))
  (bind _returnvalue (Transformation|GetRelativeTransform _button4))
  (Variables|Default|SetOut%20Position4 (Math|Transform|MakeTransform (.location _returnvalue) (.rotation _returnvalue) (.scale _returnvalue)))
  (Variables|Default|SetIn%20Position4 (Math|Transform|MakeTransform (- (.location _returnvalue) "0.000000,10.000000,0.000000") (.rotation _returnvalue) (.scale _returnvalue)))
  (Input|EnableInput (Game|GetPlayerController 0)))

(event Input|ActionEvents|InputActionInteract
  (params (Key :type Key%20Structure :default "None"))
  ;[1 1 1] Button Interaction
  (:Pressed
    (Utilities|FlowControl|Gate true
      (:Exit
        (Audio|PlaySoundatLocation "/Game/Assets/Buttons/Button_Click_-_Trim.Button_Click_-_Trim" (Transformation|GetActorLocation) "0, 0, 0" 1.0 1.0 0.0 0 0 0 0)
        ;[1 1 1] Button Animation
        (bind _button_in2 (Timeline|Button%20In PlayFromStart)
          (:Update
            (Transformation|SetRelativeTransform (Variables|Default|GetButton4) (Math|Transform|Lerp(Transform) (Variables|Default|GetOut%20Position4) (Variables|Default|GetIn%20Position4) _button_in2) false false))
          (:Finished
            (bind _button_in2_2 (Timeline|Button%20Out ReverseFromEnd)
              (:Update
                (Transformation|SetRelativeTransform (Variables|Default|GetButton4) (Math|Transform|Lerp(Transform) (Variables|Default|GetOut%20Position4) (Variables|Default|GetIn%20Position4) _button_in2_2) false false)
                ;[1 1 1] Open Door w/ Button
                (bind _outactors (Actor|GetAllActorsOfClass "/Game/Assets/Buttons/Door4_BP.Door4_BP_C"))
                (bind _array_element (Utilities|Array|ForEachLoopwithBreak _outactors)
                  (:LoopBody
                    (if (== (Variables|/Game/Assets/Buttons/Door4_BP.Door4_BP_C|GetDoor4%20Value _array_element) (Variables|Default|GetButton4%20Value))
                      (Default|OpenDoor4 _array_element))))))))))))

(fn ConstructionScript)